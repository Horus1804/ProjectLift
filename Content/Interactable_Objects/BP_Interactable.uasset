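; Interactable elevator actor that opens its lift and elevator doors on interaction, then closes them automatically.
; The Interactions event drives both door pairs with one timeline lerp over shared location variables, then reverses it after a delay behind a DoOnce.
; The construction script picks the shaft mesh from an enum, and GetAttachTransform returns the AttachPoint's world transform.
; Floor-destination logic is unconnected and AddIKGoals is empty.
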(event EventBeginPlay
  (Variables|Default|SetNbrs_Etages 0))

(event Collision|EventActorBeginOverlap
  (params (OtherActor :type Actor%20Object%20Reference)))

(event EventTick
  (params (DeltaSeconds :type Float%20%28single-precision%29)))

(event EventInteractions
  ;[0 0.1229 1] Ouverture/Fermeture des portes de l'ascenseur
  (Variables|Door_Location|SetDoor_01_Initial_Location (Variables|/Script/Engine.SceneComponent|GetRelativeLocation (Variables|Default|GetLift_Door_01)))
  (Variables|Door_Location|SetDoor_02_Initial_Location (Variables|/Script/Engine.SceneComponent|GetRelativeLocation (Variables|Default|GetLift_Door_02)))
  (Variables|Door_Location|SetDoor_01_Initial_Location (Variables|/Script/Engine.SceneComponent|GetRelativeLocation (Variables|Default|GetElevator_Door_01)))
  (Variables|Door_Location|SetDoor_02_Initial_Location (Variables|/Script/Engine.SceneComponent|GetRelativeLocation (Variables|Default|GetElevator_Door_02)))
  (Utilities|FlowControl|Sequence
    (:then_0
      (bind _alpha (Timeline|Door_Timeline Play)
        (:Update
          (Variables|Default|SetTimeline_Alpha _alpha)
          (Transformation|SetRelativeLocation (Variables|Default|GetLift_Door_01) (Math|Vector|Lerp(Vector) (Variables|Door_Location|GetDoor_01_Initial_Location) (Variables|Door_Location|GetDoor_01_Final_Location) (Variables|Default|GetTimeline_Alpha)) false false)
          (Transformation|SetRelativeLocation (Variables|Default|GetLift_Door_02) (Math|Vector|Lerp(Vector) (Variables|Door_Location|GetDoor_02_Initial_Location) (Variables|Door_Location|GetDoor_02_Final_Location) (Variables|Default|GetTimeline_Alpha)) false false)
          (Transformation|SetRelativeLocation (Variables|Default|GetElevator_Door_01) (Math|Vector|Lerp(Vector) (Variables|Door_Location|GetDoor_01_Initial_Location) (Variables|Door_Location|GetDoor_01_Final_Location) (Variables|Default|GetTimeline_Alpha)) false false)
          (Transformation|SetRelativeLocation (Variables|Default|GetElevator_Door_02) (Math|Vector|Lerp(Vector) (Variables|Door_Location|GetDoor_02_Initial_Location) (Variables|Door_Location|GetDoor_02_Final_Location) (Variables|Default|GetTimeline_Alpha)) false false))
        (:Finished
          (Utilities|FlowControl|Delay 5.0)
          (Utilities|FlowControl|DoOnce false :!label _label
            (:Completed
              (Timeline|Door_Timeline ReverseFromEnd))))))
    (:then_1
      (goto _label Reset))))

(fn ConstructionScript
  (Components|StaticMesh|SetStaticMesh (Variables|Default|GetLift_shaft) (Utilities|Select :Index (Variables|Default|GetEnum) :NewEnumerator0 "/Game/Lift/Meshes/SM_Lift01Shaft01.SM_Lift01Shaft01")))

(fn AddIKGoals
  (return 0))

(fn GetAttachTransform
  (return (Transformation|GetWorldTransform (Variables|Default|GetAttach_Point))))